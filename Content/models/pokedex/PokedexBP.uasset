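; Pokedex actor that detects Pokemon in the world and tells a camera Blueprint to display them.
; When an actor tagged Pokemon begins overlapping its capsule, it passes that actor to PokemonCameraBP to show.
; A ClearPokedex event, bound at BeginPlay, tells the camera to hide the Pokemon.
; Both show and hide act only when PokedexCameraSet is true.
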(event OnComponentBeginOverlap(Capsule)
  (params (OverlappedComponent :type Primitive%20Component%20Object%20Reference) (OtherActor :type Actor%20Object%20Reference) (OtherComp :type Primitive%20Component%20Object%20Reference) (OtherBodyIndex :type Integer) (bFromSweep :type Boolean) (SweepResult :type Hit%20Result%20Structure%20%28by%20ref%29))
  (if (Variables|Default|GetPokedexCameraSet)
    (if (Actor|ActorHasTag OtherActor "Pokemon")
      (Default|ShowPokemonEvent (Variables|Default|GetPokemonCameraBP) OtherActor))))

(event Custom|ClearPokedex_Event
  (if (Variables|Default|GetPokedexCameraSet)
    (Default|HidePokemonEvent (Variables|Default|GetPokemonCameraBP))))

(event EventBeginPlay
  (EventDispatchers|BindEventtoClearPokedex (delegate Custom|ClearPokedex_Event)))

(event Collision|EventActorBeginOverlap
  (params (OtherActor :type Actor%20Object%20Reference)))

(event EventTick
  (params (DeltaSeconds :type Float%20%28single-precision%29)))

(fn ConstructionScript)