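; Pokémon inventory actor that builds an in-world list of Pokémon, seeded on BeginPlay with a hardcoded Bulbasaur.
; BeginPlay binds show, hide and add-Pokéball events; show and hide toggle only the root's visibility, without propagating to children.
; AddPokeballToList spawns mesh and text components for ball, name and level at fixed offsets.
; The add event, marked TODO, stores the ball and creates a zero-scale mesh component without updating the list.
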(event OnComponentHit(Cube)
  (params (HitComponent :type Primitive%20Component%20Object%20Reference) (OtherActor :type Actor%20Object%20Reference) (OtherComp :type Primitive%20Component%20Object%20Reference) (NormalImpulse :type Vector :default "0, 0, 0") (Hit :type Hit%20Result%20Structure%20%28by%20ref%29)))

(event Custom|ShowInventory_Event
  (Rendering|SetVisibility (Variables|Default|GetDefaultSceneRoot) true false))

(event Custom|AddPokeball_Event
  (params (Pokeball :type Pokeball%20BP%20Object%20Reference))
  ;[1 1 1] TODO delete pokeball en scalen enzo....
  (bind _returnvalue (Utilities|Array|Add (Variables|Default|GetPokeballs) Pokeball))
  (bind _returnvalue_2 (AddComponent|AddStaticMeshComponent Pokeball false (Math|Transform|MakeTransform "0,20.000000,20.000000" "0, 0, 0" "0, 0, 0")))
  (Components|StaticMesh|SetStaticMesh _returnvalue_2 "/Game/models/pokeball/pokeball.pokeball"))

(event Custom|HideInventory_Event
  (Rendering|SetVisibility (Variables|Default|GetDefaultSceneRoot) false false))

(event EventBeginPlay
  (Utilities|FlowControl|Sequence
    (:then_0
      (EventDispatchers|BindEventtoShowInventory (delegate Custom|ShowInventory_Event)))
    (:then_1
      (EventDispatchers|BindEventtoHideInventory (delegate Custom|HideInventory_Event)))
    (:then_2
      (EventDispatchers|BindEventtoAddPokeball (delegate Custom|AddPokeball_Event)))
    (:then_3
      (CallFunction|AddPokeballtoList (Utilities|Struct|MakePokemonStruct "Bulbasaur" 8 253 45 50)))))

(event Collision|EventActorBeginOverlap
  (params (OtherActor :type Actor%20Object%20Reference)))

(event EventTick
  (params (DeltaSeconds :type Float%20%28single-precision%29)))

(fn ConstructionScript)

(fn AddPokeballtoList
  (params (PokemonData :type Pokemon%20Struct%20Structure))
  (bind _returnvalue (Math|Vector|MakeVector 0.0 -25.0 25.0))
  (LocalVariables|SetPokemonDataVar PokemonData)
  (Utilities|FlowControl|Sequence
    (:then_0
      ;[1 1 1] Show Pokeball
      (bind _returnvalue_2 (AddComponent|AddStaticMeshComponent false (Math|Transform|MakeTransform _returnvalue "0.000000,90.000000, 0" "0.500000,0.500000,0.500000")))
      (Components|StaticMesh|SetStaticMesh _returnvalue_2 "/Game/models/pokeball/pokeball.pokeball"))
    (:then_1
      ;[1 1 1] Show Name
      (bind _returnvalue_3 (AddComponent|AddTextRenderComponent false (Math|Transform|MakeTransform (+ _returnvalue "0,8.000000,-1.000000") "0,180.000000, 0" "0.500000,0.500000,0.500000")))
      (Rendering|Components|TextRender|SetText _returnvalue_3 (Utilities|Text|ToText(String) (.Name (Utilities|Struct|BreakPokemonStruct (LocalVariables|GetPokemonDataVar))))))
    (:then_2
      ;[1 1 1] Show Lvl
      (bind _returnvalue_4 (AddComponent|AddTextRenderComponent false (Math|Transform|MakeTransform (+ _returnvalue "0,45.000000,-1.000000") "0,180.000000, 0" "0.500000,0.500000,0.500000")))
      (Rendering|Components|TextRender|SetText _returnvalue_4 (Utilities|Text|ToText(String) (Utilities|String|Append "Lv" (Utilities|String|ToString(Integer) (.Lvl (Utilities|Struct|BreakPokemonStruct (LocalVariables|GetPokemonDataVar))))))))))