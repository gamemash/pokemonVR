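; Pokeball actor that, when it hits a Pokemon-tagged actor, makes a weighted random catch roll and stores the Pokemon's data.
; A catch runs a timeline that bumps the ball, freezes it facing the Pokemon, applies an interaction material and beam, then drops it and destroys the Pokemon.
; CatchPokemon rolls separately for storing and returning success.
; Custom-depth highlight events are included; rescale binding is unconnected and PickupBall is empty.
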(event OnComponentHit(pokeball)
  (params (HitComponent :type Primitive%20Component%20Object%20Reference) (OtherActor :type Actor%20Object%20Reference) (OtherComp :type Primitive%20Component%20Object%20Reference) (NormalImpulse :type Vector) (Hit :type Hit%20Result%20Structure%20%28by%20ref%29))
  (bind _pokeball (Variables|Default|Getpokeball))
  (bind _pokeball_2 (Variables|Default|Getpokeball))
  (bind _pokeball_3 (Variables|Default|Getpokeball))
  (if (Actor|ActorHasTag OtherActor "Pokemon")
    (bind _success (CallFunction|CatchPokemon OtherActor))
    (if _success
      (Timeline|Timeline_1 PlayFromStart
        (:BumpIt
          ;[1 1 1] Bump the pokeball up
          (Physics|SetPhysicsLinearVelocity _pokeball_3 (* (Math|Vector|CrossProduct (Math|Vector|Normalize (- (Transformation|GetActorLocation OtherActor) (Transformation|GetActorLocation (Variables|Default|GetPlayer)))) "0,1.000000,-1.000000") 5e+02) false "None")
          (Collision|SetCollisionEnabled _pokeball_3 "PhysicsOnly"))
        (:StartAnimation
          (Utilities|FlowControl|Sequence
            (:then_0
              ;[1 1 1] Stop Pokeball and look at pokemon
              (Physics|SetSimulatePhysics _pokeball_2 false)
              (Transformation|SetWorldRotation _pokeball_2 (Math|Rotator|FindLookatRotation (Transformation|GetWorldLocation _pokeball_2) (Transformation|GetActorLocation (Variables|Default|GetPokemon))) false false))
            (:then_1
              ;[1 1 1] Highlight Pokemon
              (bind _asmesh_component (Utilities|Casting|CastToMeshComponent (VehicleSound|GetRootComponent (Variables|Default|GetPokemon))))
              (for (_ _array_index) (Rendering|Material|GetMaterials _asmesh_component)
                (Rendering|Material|SetMaterial _asmesh_component _array_index "/Game/models/pokeball/Mat_PokemonPokeballInteraction.Mat_PokemonPokeballInteraction")))
            (:then_2
              ;[1 1 1] Create Beam to pokemon
              (bind _returnvalue (Effects|SpawnEmitteratLocation "/Game/models/pokeball/P_Beam.P_Beam" (Transformation|GetActorLocation (Variables|Default|GetPokemon))))
              (Effects|Components|ParticleSystem|SetVectorParameter _returnvalue "TargetLocation" (Transformation|GetWorldLocation (Variables|Default|Getpokeball))))))
        (:Done
          ;[1 1 1] Remove beam, pokemon and drop the ball
          (Utilities|FlowControl|Sequence
            (:then_0
              (Physics|SetSimulatePhysics _pokeball true)
              (Collision|SetCollisionEnabled _pokeball "QueryAndPhysics"))
            (:then_1
              (Components|DestroyComponent _returnvalue)
              (Actor|DestroyActor (Variables|Default|GetPokemon)))))))))

(event Custom|BallThrown_Event
  (params (Player :type VR%20Player%20Pawn%20Object%20Reference))
  (Variables|Default|SetPlayer Player))

(event Custom|RescaleBall_Event
  (params (beginScale :type Float%20%28single-precision%29) (endScale :type Float%20%28single-precision%29))
  (bind _pokeballsize (Timeline|GrowingTimeline Play)
    (:Update
      (Transformation|SetActorScale3D (Math|Conversions|ToVector(Float) (+ (* (- endScale beginScale) _pokeballsize) beginScale))))))

(event EventBeginPlay
  (Utilities|FlowControl|Sequence
    (:then_0
      (EventDispatchers|BindEventtoBallThrown (delegate Custom|BallThrown_Event)))))

(event EventTick
  (params (DeltaSeconds :type Float%20%28single-precision%29)))

(event EventDeHightlightActor
  (Rendering|SetRenderCustomDepth (Variables|Default|Getpokeball) false))

(event EventHighlightActor
  (Rendering|SetRenderCustomDepth (Variables|Default|Getpokeball) true))

(event EventHighlightActorRemote
  (Rendering|SetRenderCustomDepth (Variables|Default|Getpokeball) true))

(event EventDeHighlightActorRemote
  (Rendering|SetRenderCustomDepth (Variables|Default|Getpokeball) false))

(fn ConstructionScript)

(fn CatchPokemon
  (params (PokemonBP :type Actor%20Object%20Reference))
  (bind _returnvalue (Math|Random|RandomBoolwithWeight 0.9))
  (if _returnvalue
    (bind _output_get (Variables|Default|SetPokemon PokemonBP))
    (Variables|Default|SetCaughtPokemon true)
    (bind _data (Class|PokemonInterface|GetData(Message) _output_get))
    (Variables|Default|SetPokemonData _data))
  (return _returnvalue))

(fn PickupBall
  (return 0))